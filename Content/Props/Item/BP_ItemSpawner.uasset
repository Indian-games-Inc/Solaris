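; Item spawner prop that places an item of a configurable class at its spawn point and replaces it after it is destroyed.
; SpawnActor creates the item with itself as owner and stores it in ItemRef, running from both the Construction Script and BeginPlay without clearing any earlier instance.
; The item's OnDestroyed event triggers Respawn, which waits RespawnDelay, spawns a replacement and rebinds to it, repeating the cycle.
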(event `self.ReceiveBeginPlay`
  (bind _itemref (`self.ItemRef`))
  (`self.SpawnActor`)
  (if (`KismetSystemLibrary.IsValid` _itemref)
    (add `self.OnDestroyed` _itemref (delegate `Respawn`))))

(event `Respawn`
  (params (DestroyedActor :type "Actor Object Reference"))
  (`KismetSystemLibrary.Delay` (`self.Respawn Delay`))
  (`self.SpawnActor`)
  (add `self.OnDestroyed` (`self.ItemRef`) (delegate `Respawn`)))

(fn `SpawnActor`
  (bind _returnvalue (`|SpawnActorFromClass` (`self.ItemClass`) (`SceneComponent.K2_GetComponentToWorld` (`self.SpawnPoint`)) "Undefined" "MultiplyWithRoot" self null))
  (set `self.ItemRef` _returnvalue))

(fn `UserConstructionScript`
  (`self.SpawnActor`))