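; BP_SecurityMonitor is a CCTV monitor prop whose unfinished or disabled logic targets showing a security camera feed on its screen.
; BeginPlay and the construction script are empty, so the setup chain never runs.
; That disconnected chain creates an M_SecurityCamera dynamic material and a viewport-sized render target scaled by camera quality.
; It sets the capture's TextureTarget to None rather than that target, then feeds it to the material with zero brightness.
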(event `self.ReceiveBeginPlay`)

(fn `UserConstructionScript`)