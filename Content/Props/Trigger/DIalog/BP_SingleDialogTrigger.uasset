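; BP_SingleDialogTrigger is a trigger prop that shows a dialog subtitle when the player overlaps it.
; On any actor overlap it gets a data table row from PickDialog, passes it on, then switches itself off via SwitchTrigger.
; SendDialogRowToHUD casts from player character through controller to BP_HUD and calls RedrawSubs with the row name.
; The switch-off also runs when a non-player overlaps and those casts fail.
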(event `self.ReceiveActorBeginOverlap`
  (params (OtherActor :type "Actor Object Reference"))
  ;[1 1 1] Some of this should be in C++ for sure
  (bind _returnvalue (`self.PickDialog`))
  (`self.Send Dialog Row To HUD` OtherActor _returnvalue)
  (`self.SwitchTrigger` false))

(fn `Send Dialog Row To HUD`
  (params (Object :type "Object Object Reference") (DataTableRowHandle :type "DataTableRowHandle Structure (by ref)"))
  (bind _asbp_player_character (cast `/Game/Player/BP_PlayerCharacter` Object))
  (bind _asbp_player_controller (cast `/Game/Player/BP_PlayerController` (`Pawn.GetController` _asbp_player_character)))
  (bind _asbp_hud (cast `/Game/GUI/HUD/BP_HUD` (`PlayerController.GetHUD` _asbp_player_controller)))
  (`/Game/GUI/HUD/BP_HUD.Redraw Subs` _asbp_hud (`.RowName` (break `DataTableRowHandle` DataTableRowHandle))))

(fn `UserConstructionScript`)