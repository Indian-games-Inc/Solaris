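; BP_SingleShotDialogTrigger is a dialog trigger prop that hands subtitle rows to the player HUD.
; Its SendDialogtoHUD event casts the supplied HUD to BP_HUD and calls RedrawSubs with the dialog row name.
; A separate Jopa function makes the same call, finding the HUD through player 0's character and controller.
; No overlap or single-shot logic appears in these graphs.
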(event `self.SendDialogToHUD`
  (params (HUD :type "HUD Object Reference") (DialogRowHandle :type "DataTableRowHandle Structure"))
  (bind _asbp_hud (cast `/Game/GUI/HUD/BP_HUD` HUD))
  (`/Game/GUI/HUD/BP_HUD.Redraw Subs` _asbp_hud (`.RowName` (break `DataTableRowHandle` DialogRowHandle))))

(fn `Jopa`
  (params (DataTableRowHandle :type "DataTableRowHandle Structure (by ref)"))
  (bind _asbp_player_character (cast `/Game/Player/BP_PlayerCharacter` (`GameplayStatics.GetPlayerCharacter` 0)))
  (bind _asbp_player_controller (cast `/Game/Player/BP_PlayerController` (`Pawn.GetController` _asbp_player_character)))
  (bind _asbp_hud (cast `/Game/GUI/HUD/BP_HUD` (`PlayerController.GetHUD` _asbp_player_controller)))
  (`/Game/GUI/HUD/BP_HUD.Redraw Subs` _asbp_hud (`.RowName` (break `DataTableRowHandle` DataTableRowHandle))))

(fn `UserConstructionScript`)