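; BP_CryptRaiderCharacter is the player character Blueprint that routes input actions to its picking, inventory and grabbing components.
; Pressing PickUp asks Picker for an item and adds it to Inventory when its name is not empty.
; Pressing and releasing Grab calls Grab and Release on Grabber.
; The Inventory action prints the names of stored items as strings, with no other display in this graph.
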(event `InputAction|Inventory`
  (params (Key :type "Key Structure"))
  (:`Pressed`
    (bind _returnvalue (`Inventory.GetInventoryItems` (`self.Inventory`)))
    (for _array_element _returnvalue
      (`KismetSystemLibrary.PrintString` (`.Name` (break `ItemData` _array_element))))))

(event `InputAction|PickUp`
  (params (Key :type "Key Structure"))
  (:`Pressed`
    (bind _returnvalue (`Picker.PickItem` (`self.Picker`)))
    (if (not (`KismetStringLibrary.IsEmpty` (`.Name` (break `ItemData` _returnvalue))))
      (`Inventory.AddItem` (`self.Inventory`) _returnvalue))))

(event `InputAction|Grab`
  (params (Key :type "Key Structure"))
  (bind _grabber (`self.Grabber`))
  (:`Pressed`
    (`Grabber.Grab` _grabber))
  (:`Released`
    (`Grabber.Release` _grabber)))

(fn `UserConstructionScript`)