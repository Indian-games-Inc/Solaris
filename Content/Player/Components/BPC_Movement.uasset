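; Player movement component that handles sprinting and stamina by switching the owning character's max walk speed between walk and sprint values.
; Initialize stores the character, applies walk speed and fills stamina.
; Sprinting starts only with stamina left and runs a looping timer that drains it, stopping automatically at the minimum.
; Stopping starts a second looping timer that restores stamina until full, and each state clears the other's timer.
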(event `StartSprinting`
  (`KismetSystemLibrary.K2_ClearAndInvalidateTimerHandle` (stale `Stop Sprint` _returnvalue))
  (if (> (`self.CurrentStamina`) 0.0)
    (`self.Set Max walk Speed` (`self.SprintSpeed`))
    (bind _returnvalue (`KismetSystemLibrary.K2_SetTimerDelegate` (delegate `Sprint Update`) (`self.StaminaConsumptionRate`) true))))

(event `Sprint Update`
  (set `self.CurrentStamina` (`KismetMathLibrary.FClamp` (- (`self.CurrentStamina`) (`self.StaminaConsumption`)) (`self.MinStamina`) (`self.MaxStamina`)))
  (if (<= (`self.CurrentStamina`) (`self.MinStamina`))
    (`self.Stop Sprint`)))

(event `Stop Sprint`
  (`KismetSystemLibrary.K2_ClearAndInvalidateTimerHandle` (stale `StartSprinting` _returnvalue))
  (`self.Set Max walk Speed` (`self.WalkSpeed`))
  (bind _returnvalue (`KismetSystemLibrary.K2_SetTimerDelegate` (delegate `Restore Stamina`) (`self.StaminaRestorationRate`) true)))

(event `Restore Stamina`
  (bind _output_get (set `self.CurrentStamina` (`KismetMathLibrary.FClamp` (+ (`self.CurrentStamina`) (`self.StaminaRestoration`)) (`self.MinStamina`) (`self.MaxStamina`))))
  (if (>= _output_get (`self.MaxStamina`))
    (`KismetSystemLibrary.K2_ClearAndInvalidateTimerHandle` (stale `Stop Sprint` _returnvalue))))

(fn `Initialize`
  (params (Character :type "BaseCharacter Object Reference"))
  (set `self.Character` Character)
  (`self.Set Max walk Speed` (`self.WalkSpeed`))
  (set `self.CurrentStamina` (`self.MaxStamina`)))

(fn `Set Max walk Speed`
  (params (MaxWalkSpeed :type "Float (single-precision)"))
  (set `CharacterMovementComponent.MaxWalkSpeed` MaxWalkSpeed (`Character.CharacterMovement` (`self.Character`))))