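; Player controller that owns the inventory screen and feeds player state to the HUD.
; On begin play it creates a hidden inventory widget, initializes the inventory items and caches the HUD.
; Input toggles the inventory with cursor and input mode, and scroll switches hotbar slots.
; Tick polls the character to update health, stamina and pin-lock hint, creating a new hint widget every frame while in pin lock.
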(event `self.ReceiveBeginPlay`
  (bind _inventorywidget (`self.InventoryWidget`))
  ;[1 0.4306 0.2964] On init event
  (`WidgetBlueprintLibrary.SetInputMode_GameOnly` self)
  (bind _returnvalue (`|CreateWidget` "/Game/GUI/Inventory/BPW_Inventory.BPW_Inventory_C" null null))
  (set `self.InventoryWidget` _returnvalue)
  (`Inventory.InitItemsArray` (`self.Inventory`))
  (`UserWidget.AddToViewport` _inventorywidget 0)
  (`Widget.SetVisibility` _inventorywidget "Hidden")
  (bind _asbp_hud (cast `/Game/GUI/HUD/BP_HUD` (`self.GetHUD`)))
  (set `self.HUD` _asbp_hud))

(event `EnhancedInput|/Game/Input/Actions/IA_Show_Inventory`
  (params (ActionValue :type Boolean) (ElapsedSeconds :type "Float (double-precision)") (TriggeredSeconds :type "Float (double-precision)") (InputAction :type "InputAction Object Reference" :default "/Game/Input/Actions/IA_Show_Inventory.IA_Show_Inventory"))
  ;[1 1 1] On Inventory show
  (:`Started`
    (`/Engine/EditorBlueprintResources/StandardMacros.FlipFlop`
      (:`A`
        (bind _inventorywidget (`self.InventoryWidget`)
          (:`then`
            (`Widget.SetVisibility` _inventorywidget "Visible")
            (`WidgetBlueprintLibrary.SetInputMode_GameAndUIEx` self null)
            (set `self.bShowMouseCursor` true))
          (:`else`)))
      (:`B`
        (bind _inventorywidget_2 (`self.InventoryWidget`)
          (:`then`
            (`Widget.SetVisibility` _inventorywidget_2 "Hidden")
            (`WidgetBlueprintLibrary.SetInputMode_GameOnly` self)
            (set `self.bShowMouseCursor` false))
          (:`else`))))))

(event `self.ReceiveTick`
  (params (DeltaSeconds :type "Float (single-precision)"))
  ;[0.2068 0.2491 0.5927] Tick event | Udate stats
  (`self.Update Health Info`)
  (`self.Update Stamina Info`)
  (`self.Update PinLock Message`))

(event `EnhancedInput|/Game/Input/Actions/IA_ScrollDown`
  (params (ActionValue :type Boolean) (ElapsedSeconds :type "Float (double-precision)") (TriggeredSeconds :type "Float (double-precision)") (InputAction :type "InputAction Object Reference" :default "/Game/Input/Actions/IA_ScrollDown.IA_ScrollDown"))
  ;[1 1 1] How to merge in a single one ???
  (:`Triggered`
    (`/Game/GUI/HUD/BP_HUD.SwitchActiveHotBarSlot` (`self.HUD`) -1)))

(event `EnhancedInput|/Game/Input/Actions/IA_ScrollUp`
  (params (ActionValue :type Boolean) (ElapsedSeconds :type "Float (double-precision)") (TriggeredSeconds :type "Float (double-precision)") (InputAction :type "InputAction Object Reference" :default "/Game/Input/Actions/IA_ScrollUp.IA_ScrollUp"))
  ;[1 1 1] How to merge in a single one ???
  (:`Triggered`
    (`/Game/GUI/HUD/BP_HUD.SwitchActiveHotBarSlot` (`self.HUD`) 1)))

(event `Update Health Info`
  (bind _asbase_character (cast `BaseCharacter` (`GameplayStatics.GetPlayerCharacter` 0)))
  (`/Game/GUI/HUD/BP_HUD.Update Health Info` (`self.HUD`) (`Health.GetHealthPercent` (`BaseCharacter.Health` _asbase_character))))

(event `Update Stamina Info`
  (bind _asbase_character (cast `BaseCharacter` (`GameplayStatics.GetPlayerCharacter` 0)))
  (`/Game/GUI/HUD/BP_HUD.Update Stamina Info` (`self.HUD`) (`Movement.GetStaminaPercent` (`BaseCharacter.Movement` _asbase_character))))

(event `Update PinLock Message`
  (bind _asbase_character (cast `BaseCharacter` (`GameplayStatics.GetPlayerCharacter` 0)))
  (if (`BaseCharacter.IsInPinLock` _asbase_character)
    (bind _returnvalue (`|CreateWidget` "/Game/GUI/PinLock/BPW_PinCodeHint.BPW_PinCodeHint_C"))
    (`/Game/GUI/HUD/BP_HUD.Update Additional Hint Info` (`self.HUD`) _returnvalue)
    (else
      (`/Game/GUI/HUD/BP_HUD.Update Additional Hint Info` (`self.HUD`) null))))

(fn `UserConstructionScript`)