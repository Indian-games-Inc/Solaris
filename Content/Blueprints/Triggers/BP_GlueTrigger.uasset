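; Trigger volume that "glues" the first overlapping actor of a configurable class while the player's grabber holds nothing.
; On tick it stores that actor and moves it one VInterpTo step toward an offset from the root, releasing it once the player grabs it.
; The construction script sizes and shows or hides the glue and freeze boxes.
; Ladder-specific delayed physics freezing is unwired, and a debug print remains.
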(event `self.ReceiveBeginPlay`
  ;[1 1 1] On init
  (bind _asbp_player_character (cast `/Game/Character/BP_PlayerCharacter` (`GameplayStatics.GetPlayerPawn` 0)))
  (bind _grabber (`/Game/Character/BP_PlayerCharacter.GetGrabber` _asbp_player_character))
  (set `self.Grabber` _grabber)
  (set `self.IsGlued` false))

(event `self.ReceiveTick`
  (params (DeltaSeconds :type "Float (single-precision)"))
  ;[1 0.8236 0.4071] Is player grabbing anything?
  (bind _returnvalue (`Grabber.IsGrabbing` (`self.Grabber`)))
  (if _returnvalue
    ;[0.2502 0.5564 1] It's selected-glued item? If so, clear it from glue
    (bind _returnvalue_2 (`self.IsSelectedItemEqualGrabbed`))
    (if _returnvalue_2
      (set `self.IsGlued` false)
      (set `self.SelectedItem` null))
    (else
      ;[1 0.5046 0.748] Is object overlapping area?
      (if (not (`self.IsGlued`))
        (bind _output (`self.SelectOverlappingItem`))
        (bind _output_get (set `self.SelectedItem` _output))
        (`self.SelectedItem`
          (:`then`
            (set `self.IsGlued` true)
            (`KismetSystemLibrary.PrintString` "Hello")
            (`self.K2_SetActorRelativeTransform` _output_get (`KismetMathLibrary.Conv_VectorToTransform` (`KismetMathLibrary.VInterpTo` (`self.K2_GetActorLocation` _output_get) (+ (`SceneComponent.K2_GetComponentLocation` (`self.DefaultSceneRoot`)) (0.0 -250.0 0.0)) DeltaSeconds 60.0)) false false))
          (:`else`))))))

(fn `IsSelectedItemEqualGrabbed`
  (returns (ReturnValue :type Boolean))
  (return (== (`ActorComponent.GetOwner` (`Grabber.GetGrabbedItem` (`self.Grabber`))) (`self.SelectedItem`))))

(fn `SelectOverlappingItem`
  (returns (Output :type "Actor Object Reference"))
  (return (`|GetArrayItem` (`self.GetOverlappingActors` (`self.Class`)))))

(fn `UserConstructionScript`
  (`BoxComponent.SetBoxExtent` (`self.GlueArea`) (`self.GlueSize`) true)
  (`BoxComponent.SetBoxExtent` (`self.FreezeArea`) (`self.FreezeSize`) true)
  (`SceneComponent.SetHiddenInGame` (`self.FreezeArea`) (not (`self.IsFrameShown`)) false)
  (`SceneComponent.SetHiddenInGame` (`self.GlueArea`) (not (`self.IsFrameShown`)) false))