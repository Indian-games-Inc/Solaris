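; BP_ItemPreview is an inventory GUI actor that renders a rotating 3D preview of an item's static mesh.
; Each tick it slowly yaws its scene component and restricts its SceneCaptureComponent2D to show only the CurrentModel mesh component.
; SetModel and ClearModel swap or empty the static mesh on CurrentModel.
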(event `self.ReceiveTick`
  (params (DeltaSeconds :type "Float (single-precision)"))
  ;[1 1 1] Rotation
  (`SceneComponent.K2_AddLocalRotation` (`self.Scene`) (`KismetMathLibrary.MakeRotator` 0.0 0.0 (* DeltaSeconds 10.0)) false false)
  ;[1 1 1] Capture only a model
  (`SceneCaptureComponent.ShowOnlyComponent` (`self.SceneCaptureComponent2D`) (`self.CurrentModel`)))

(fn `ClearModel`
  (`StaticMeshComponent.SetStaticMesh` (`self.CurrentModel`) null))

(fn `SetModel`
  (params (Model :type "StaticMesh Object Reference"))
  (`StaticMeshComponent.SetStaticMesh` (`self.CurrentModel`) Model))

(fn `UserConstructionScript`)